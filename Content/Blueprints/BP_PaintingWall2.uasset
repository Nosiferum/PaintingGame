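; BP_PaintingWall2 is a paintable wall that records drawing into the PaintingTarget render target.
; The target is cleared to black on BeginPlay, and again every tick while IsErasable is true.
; DrawOnWall passes a 2D location to the material instance's DrawLocation parameter, then draws that material into the target.
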(event Custom|DrawOnWall
  (params (Location%20To%20Draw :type Vector%202D%20Structure))
  (bind _mymaterialinstance (Variables|Default|GetMyMaterialInstance))
  (Rendering|Material|SetVectorParameterValue _mymaterialinstance "DrawLocation" (Math|Conversions|ToLinearColor(Vector) (Math|Conversions|ToVector(Vector2D) Location%20To%20Draw)) :!class /Script/Engine.MaterialInstanceDynamic)
  (Rendering|DrawMaterialtoRenderTarget "/Game/Materials/PaintingTarget.PaintingTarget" _mymaterialinstance))

(event EventTick
  (params (DeltaSeconds :type Float%20%28single-precision%29))
  (if (Variables|Default|GetIsErasable)
    (Rendering|ClearRenderTarget2D "/Game/Materials/PaintingTarget.PaintingTarget")))

(event EventBeginPlay
  (Rendering|ClearRenderTarget2D "/Game/Materials/PaintingTarget.PaintingTarget"))

(fn ConstructionScript)